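; Cel-shading outline Blueprint that draws a configurable outline around a skeletal mesh using a duplicate mesh component.
; DuplicateMesh, run on construction and BeginPlay, applies the chosen mesh and optional material, then spawns an unattached copy at its world transform.
; The copy uses a custom outline mesh if valid, otherwise the same mesh.
; A dynamic M_Outline instance on one material slot receives color, thickness, intensity and distance-scaling settings.
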(event `self.ReceiveBeginPlay`
  (`self.DuplicateMesh`))

(fn `DuplicateMesh`
  (`SkinnedMeshComponent.SetSkinnedAssetAndUpdate` (`self.SkeletalMesh`) (`self.Your Mesh Skeletal`) true)
  (`/Engine/EditorBlueprintResources/StandardMacros.IsValid` (`self.Material`)
    (:`Is Valid`
      (`PrimitiveComponent.SetMaterial` (`self.SkeletalMesh`) (`self.Material Index`) (`self.Material`)))
    (:`Is Not Valid`
      _))
  (`/Engine/EditorBlueprintResources/StandardMacros.IsValid` (`self.Outline Mesh Skeletal`)
    (:`Is Valid`
      ;[1 1 1] Outline Mesh
      (bind _returnvalue (`AddComponent|NODE_AddSkeletalMeshComponent-1` :`bManualAttachment` true :`RelativeTransform` (`SceneComponent.K2_GetComponentToWorld` (`self.SkeletalMesh`))))
      (bind _output_get (set `self.Skeletal Mesh Component` _returnvalue))
      (`SkinnedMeshComponent.SetSkinnedAssetAndUpdate` _output_get (`self.Outline Mesh Skeletal`) true)
      ;[1 1 1] Outline Parameters for generated mesh
      (bind _returnvalue_2 (`PrimitiveComponent.CreateDynamicMaterialInstance` _output_get (`self.Material Index`) "/Game/Assets/CartoonCelShader/Materials/CelShader/M_Outline.M_Outline" "None"))
      (`|ExecutionSequence`
        (:`then_0`
          (`MaterialInstanceDynamic.SetVectorParameterValue` _returnvalue_2 "Outline Color" (`self.Outline Color`)))
        (:`then_1`
          (`MaterialInstanceDynamic.SetScalarParameterValue` _returnvalue_2 "Outline Thickness" (`self.Outline Thickness`))
          (`MaterialInstanceDynamic.SetScalarParameterValue` _returnvalue_2 "Outline Intensity" (`self.Outline Intensity`)))
        (:`then_2`
          (if (`self.Outline shrink over distance`)
            (`MaterialInstanceDynamic.SetScalarParameterValue` _returnvalue_2 "OutlineScaleOverDistance" 0.0)
            (else
              (`MaterialInstanceDynamic.SetScalarParameterValue` _returnvalue_2 "OutlineScaleOverDistance" 1.0))))))
    (:`Is Not Valid`
      ;[1 1 1] Automatic Outline
      (bind _returnvalue_3 (`AddComponent|NODE_AddSkeletalMeshComponent-0` :`bManualAttachment` true :`RelativeTransform` (`SceneComponent.K2_GetComponentToWorld` (`self.SkeletalMesh`))))
      (bind _output_get_2 (set `self.Skeletal Mesh Component` _returnvalue_3))
      (`SkinnedMeshComponent.SetSkinnedAssetAndUpdate` _output_get_2 (`self.Your Mesh Skeletal`) true)
      ;[1 1 1] Outline Parameters
      (bind _returnvalue_4 (`PrimitiveComponent.CreateDynamicMaterialInstance` _output_get_2 (`self.Material Index`) "/Game/Assets/CartoonCelShader/Materials/CelShader/M_Outline.M_Outline" "None"))
      (`|ExecutionSequence`
        (:`then_0`
          (`MaterialInstanceDynamic.SetVectorParameterValue` _returnvalue_4 "Outline Color" (`self.Outline Color`)))
        (:`then_1`
          (`MaterialInstanceDynamic.SetScalarParameterValue` _returnvalue_4 "Outline Thickness" (`self.Outline Thickness`))
          (`MaterialInstanceDynamic.SetScalarParameterValue` _returnvalue_4 "Outline Intensity" (`self.Outline Intensity`)))
        (:`then_2`
          (if (`self.Outline shrink over distance`)
            (`MaterialInstanceDynamic.SetScalarParameterValue` _returnvalue_4 "OutlineScaleOverDistance" 0.0)
            (else
              (`MaterialInstanceDynamic.SetScalarParameterValue` _returnvalue_4 "OutlineScaleOverDistance" 1.0))))))))

(fn `UserConstructionScript`
  (`self.DuplicateMesh`))