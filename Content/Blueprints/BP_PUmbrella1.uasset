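; BP_PUmbrella1 is an actor, likely an umbrella prop, that spins its static mesh around yaw and refreshes a scene capture.
; Each Tick applies both a local and a relative yaw step, scaled by LocalRotation and delta time, then calls CaptureScene on the referenced Capture's 2D component.
; The timer-driven RotateLocalZ function, which would steadily increase LocalRotation, sits behind a RotateAlways check that never runs.
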(event `self.ReceiveBeginPlay`)

(event `self.ReceiveTick`
  (params (DeltaSeconds :type "Float (single-precision)"))
  (bind _staticmeshcomponent (`self.StaticMeshComponent`))
  (bind _returnvalue (* DeltaSeconds (`self.LocalRotation`)))
  (`SceneComponent.K2_AddLocalRotation` _staticmeshcomponent (`KismetMathLibrary.MakeRotator` 0.0 0.0 _returnvalue) false false)
  (`SceneComponent.K2_AddRelativeRotation` _staticmeshcomponent (`KismetMathLibrary.MakeRotator` 0.0 0.0 _returnvalue) false false)
  (`SceneCaptureComponent2D.CaptureScene` (`SceneCapture2D.CaptureComponent2D` (`self.Capture`))))

(fn `RotateLocalZ`
  (bind _output_get (set `self.LocalRotation` (+ (`self.LocalRotation`) (* 0.01 1.0))))
  (`SceneComponent.K2_AddRelativeRotation` (`self.StaticMeshComponent`) (`KismetMathLibrary.MakeRotator` 0.0 0.0 _output_get) false false))

(fn `UserConstructionScript`)