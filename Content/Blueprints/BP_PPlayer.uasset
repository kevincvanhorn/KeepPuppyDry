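; BP_PPlayer is a player Blueprint that changes rain in response to touch begin and end events.
; Each event plays a timeline that lerps CurRain between its current value and a fixed level, writing it to the Rain parameter of MPC_Umbrella.
; The two timelines stop each other on update, so the latest touch event takes over.
; Menu widget, start-screen hiding, rain sound and music nodes are present but never run.
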(event `self.ReceiveBeginPlay`)

(event `self.ReceiveTick`
  (params (DeltaSeconds :type "Float (single-precision)")))

(event `self.OnUTouchBegin`
  (bind (_direction _track) (`Timeline|Timeline_0` :!via `PlayFromStart` :!label _label)
    (:`Update`
      (bind _output_get (set `self.curRain` (`KismetMathLibrary.Lerp` (`self.curRain`) 0.015 _track)))
      (`KismetMaterialLibrary.SetScalarParameterValue` "/Game/Assets/BaseMaterials/MPC_Umbrella.MPC_Umbrella" "Rain" _output_get)
      (bind (_direction_2 _value) (`Timeline|Timeline_1` :!via `Stop` :!label _label_2)
        (:`Update`
          (bind _output_get_2 (set `self.curRain` (`KismetMathLibrary.Lerp` 0.03 (`self.curRain`) _value)))
          (`KismetMaterialLibrary.SetScalarParameterValue` "/Game/Assets/BaseMaterials/MPC_Umbrella.MPC_Umbrella" "Rain" _output_get_2)
          (goto _label :!via `Stop`))))))

(event `self.OnUTouchEnd`
  (goto _label_2 :!via `PlayFromStart`))

(fn `UserConstructionScript`)